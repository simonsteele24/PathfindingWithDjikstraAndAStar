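; BP_SteeringActor is a grid-pathfinding actor that builds paths based on the player's position.
; On BeginPlay it generates the grid, spawns node actors, then loops on a delay, requesting a new path when the current one is empty.
; Optional smoothing uses visibility line traces to drop redundant waypoints before setting the path.
; Tick converts actor and player locations to grid coordinates, scales a speed arrow and draws debug path spheres.
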(event EventBeginPlay
  (bind _returnvalue (Transformation|GetActorLocation))
  (bind _griddisplacement (Variables|Default|GetgridDisplacement))
  (bind _playerpos (Variables|Default|GetPlayerPos))
  (bind _returnvalue_2 (Math|Float|Truncate _griddisplacement))
  (bind (_x _y) (Math|Vector|BreakVector _returnvalue))
  ;[1 1 1] Temporarily Make the player go to itself
  (Class|PathFindingActor|GenerateGrid)
  (Variables|Default|SetTargetPos _returnvalue)
  (Variables|Default|SettempEndPos (Math|Vector2D|MakeVector2D (Math|Conversions|ToFloat(Integer) (/ (Math|Float|Round _x) _returnvalue_2)) (Math|Conversions|ToFloat(Integer) (/ (Math|Float|Round _y) _returnvalue_2))))
  ;[1 1 1] Get player object
  (bind _outactors (Actor|GetAllActorsOfClass "/Game/Misc/BP_Player.BP_Player_C"))
  (for _array_element _outactors
    (Variables|Default|SetPlayer _array_element))
  (Utilities|FlowControl|Delay 0.1)
  (CallFunction|GenerateGridNodes)
  (CallFunction|UpdateOwnPosition)
  (Utilities|FlowControl|Delay 0.1)
  ;[1 1 1] Continue to update path based on player position
  (if (== (Utilities|Array|Length (Variables|Default|GetPath)) 0) :!label _label
    (if (Variables|Default|GetreachedDestination)
      (Variables|Default|SetreachedDestination false)
      (elif (Math|Vector|Equal(Vector) (Variables|Default|GetActorPos) _playerpos 0.0001)
        (Variables|Default|SetActorPos (Variables|Default|GettempEndPos))
        (bind _returnvalue_3 (Class|PathFindingActor|FindPath (Variables|Default|GetActorPos) _playerpos))
        (if (Variables|Default|GetisSmoothing)
          (Variables|Default|SettempEndPos (Variables|Default|GetPlayerPos))
          (Variables|Default|SetinputPath _returnvalue_3)
          (CallFunction|SmoothPath)
          (else
            (Class|PathFindingActor|SetPathtoFollow _returnvalue_3))))))
  (Utilities|FlowControl|Delay 0.2)
  (goto _label))

(event EventTick
  (params (DeltaSeconds :type Float%20%28single-precision%29))
  ;[1 1 1] Update the positioning and path visualizations
  (CallFunction|UpdateOwnPosition)
  (CallFunction|FindPlayerPosition)
  (CallFunction|UpdateArrow)
  (CallFunction|DisplatPath))

(fn ConstructionScript)

(fn UpdateArrow
  (Transformation|SetRelativeScale3D (Variables|Default|GetArrow) (Math|Vector|MakeVector (Math|Float|MapRangeClamped (Math|Vector|VectorLength (Variables|Default|GetSteeringVelocity)) 0.0 (Variables|Default|GetMaxSpeed) 1.0 3.0) 2.0 3.0)))

(fn DisplatPath
  (Rendering|Debug|DrawDebugSphere (Variables|Default|GetTargetPos) 1e+02 12 "(R=0.117766,G=1.000000,B=0.143879,A=1.000000)" 0.0)
  (for _array_element (Variables|Default|GetPath)
    (Rendering|Debug|DrawDebugSphere _array_element 3e+01 12 "(R=0.356519,G=1.000000,B=0.617714,A=1.000000)" 0.0)))

(fn UpdateOwnPosition
  (bind _returnvalue (Transformation|GetActorLocation))
  (bind _griddisplacement (Variables|Default|GetgridDisplacement))
  (bind _returnvalue_2 (Math|Float|Truncate _griddisplacement))
  (bind (_x _y) (Math|Vector|BreakVector _returnvalue))
  (Variables|Default|SetActorPos (Math|Vector2D|MakeVector2D (Math|Conversions|ToFloat(Integer) (/ (Math|Float|Round _x) _returnvalue_2)) (Math|Conversions|ToFloat(Integer) (/ (Math|Float|Round _y) _returnvalue_2)))))

(fn FindPlayerPosition
  (bind _griddisplacement (Variables|Default|GetgridDisplacement))
  (bind _player (Variables|Default|GetPlayer))
  (bind _returnvalue (Transformation|GetActorLocation _player))
  (bind (_x _y) (Math|Vector|BreakVector _returnvalue))
  (Variables|Default|SetPlayerPos (Math|Vector2D|MakeVector2D (Math|Conversions|ToFloat(Integer) (Math|Float|Round (/ _x _griddisplacement))) (Math|Conversions|ToFloat(Integer) (Math|Float|Round (/ _y _griddisplacement))))))

(fn GenerateGridNodes
  (for _index (range 0 (- (Math|Float|Truncate (Variables|Default|GetgridSizeX)) 1))
    (for _index_2 (range 0 (- (Math|Float|Truncate (Variables|Default|GetgridSizeY)) 1))
      (bind _returnvalue (Class|PathFindingActor|GetGridNodePosition _index _index_2))
      (Game|SpawnActorfromClass "/Game/SteeringActor/GridNode.GridNode_C" (Math|Conversions|ToTransform(Vector) _returnvalue) "Undefined" 0 0))))

(fn ContinouslyUpdatePath)

(fn SmoothPath
  ;[1 1 1] Makes sure that the path is not 0
  (if (== (Utilities|Array|Length (Variables|Default|GetinputPath)) 0)
    (return)
    (else
      ;[1 1 1] If the path is 2, no need to smooth the path, just set the path
      (if (== (Utilities|Array|Length (Variables|Default|GetinputPath)) 2)
        (bind _output_get (Variables|Default|SetoutputPath (Variables|Default|GetinputPath)))
        (Class|PathFindingActor|SetPathtoFollow _output_get)
        ;[1 1 1] Clear the arrays after done with it
        (Utilities|Array|Clear (Variables|Default|GetinputPath))
        (Utilities|Array|Clear (Variables|Default|GetoutputPath))
        (return)
        (else
          ;[1 1 1] Add first index of the input path to the output path before loop, then set the input index to 2 because we assume two adjacent nodes will pass the raycast
          (Utilities|Array|Add (Variables|Default|GetoutputPath) (Utilities|Array|Get(acopy) (Variables|Default|GetinputPath)))
          (Variables|Default|SetinputIndex (Variables|Default|Getnumber2))
          ;[1 1 1] Basically the whole while look that makes the cast between the nodes and checks if it hit something.
          (while (< (Variables|Default|GetinputIndex) (- (Utilities|Array|Length (Variables|Default|GetinputPath)) 1))
            (bind _returnvalue (Collision|LineTraceByChannel (Utilities|Array|Get(acopy) (Variables|Default|GetoutputPath) (- (Utilities|Array|Length (Variables|Default|GetoutputPath)) 1)) (Utilities|Array|Get(acopy) (Variables|Default|GetinputPath) (Variables|Default|GetinputIndex)) "TraceTypeQuery1" false 0 "ForOneFrame"))
            (if _returnvalue
              (Utilities|Array|Add (Variables|Default|GetoutputPath) (Utilities|Array|Get(acopy) (Variables|Default|GetinputPath) (- (Variables|Default|GetinputIndex) 1))))
            (Variables|Default|SetinputIndex (+ (Variables|Default|GetinputIndex) 1)))
          ;[1 1 1] Add the end node to the output and pass in the output path to the set path function
          (Utilities|Array|Add (Variables|Default|GetoutputPath) (Utilities|Array|Get(acopy) (Variables|Default|GetinputPath) (- (Utilities|Array|Length (Variables|Default|GetinputPath)) 1)))
          (Class|PathFindingActor|SetPathtoFollow (Variables|Default|GetoutputPath))
          ;[1 1 1] Clear the arrays after done with it
          (Utilities|Array|Clear (Variables|Default|GetinputPath))
          (Utilities|Array|Clear (Variables|Default|GetoutputPath))
          (return))))))