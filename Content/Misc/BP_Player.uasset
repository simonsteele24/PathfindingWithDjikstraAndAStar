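; Player for a grid pathfinding demo, moved by left stick within the manager's grid bounds, with mouse-wheel camera zoom.
; BeginPlay adds the control UI, finds the pathfinding manager, spawns random walls and hands them to steering actors for path finding.
; Movement with a positive component makes every steering actor re-path, optionally smoothed.
; Further functions spawn steering actors off walls and toggle Dijkstra or path smoothing on all of them.
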(event EventBeginPlay
  (bind _returnvalue (Game|GetPlayerController 0))
  ;[1 1 1] Add UI to the screen
  (bind _returnvalue_2 (UserInterface|CreateWidget "/Game/Misc/BP_PathfindingControlUI.BP_PathfindingControlUI_C"))
  (UserInterface|Viewport|AddtoViewport _returnvalue_2 0)
  (Input|SetInputModeGameandUI _returnvalue 0 "DoNotLock" false)
  (Variables|/Script/Engine.PlayerController|SetbShowMouseCursor _returnvalue true)
  ;[1 1 1] Set the pathfinding Manager instance
  (bind _outactors (Actor|GetAllActorsOfClass "/Game/SteeringActor/BP_PathFindingManager.BP_PathFindingManager_C"))
  (for _array_element _outactors
    (bind _asbp_path_finding_manager (Utilities|Casting|CastToBP_PathFindingManager _array_element))
    (Variables|Default|SetPathFindingManager _asbp_path_finding_manager))
  ;[1 1 1] Spawns Walls randomly and assigns them to steering actors
  (Utilities|FlowControl|Delay 0.2)
  (CallFunction|SpawnWallsRandomly)
  (CallFunction|AssignWallstoActors))

(event EventTick
  (params (DeltaSeconds :type Float%20%28single-precision%29))
  (bind _returnvalue (Transformation|GetActorLocation))
  (bind _returnvalue_2 (Input|AxisValues|GetLeftStickX))
  (bind _returnvalue_3 (Input|AxisValues|GetLeftStickY))
  (bind _speed (Variables|Default|GetSpeed))
  (bind _pathfindingmanager (Variables|Default|GetPathFindingManager))
  (bind (_x _y) (Math|Vector|BreakVector _returnvalue))
  (bind _returnvalue_4 (Math|Vector|MakeVector _returnvalue_3 _returnvalue_2 0.0))
  (bind _griddisplacement (Variables|/Game/SteeringActor/BP_PathFindingManager.BP_PathFindingManager_C|GetGridDisplacement _pathfindingmanager))
  (bind _griddimensions (Variables|/Game/SteeringActor/BP_PathFindingManager.BP_PathFindingManager_C|GetGridDimensions _pathfindingmanager))
  (bind _returnvalue_5 (- _griddimensions 1.0))
  (bind _returnvalue_6 (* _returnvalue_4 _speed))
  (bind (_x_2 _y_2) (Math|Vector2D|BreakVector2D _returnvalue_5))
  (bind _returnvalue_7 (* _returnvalue_6 DeltaSeconds))
  (bind (_x_3 _y_3) (Math|Vector|BreakVector _returnvalue_7))
  (bind _returnvalue_8 (+ _x _x_3))
  (bind _returnvalue_9 (+ _y_3 _y))
  ;[1 1 1] Make sure that the position of the player is negative
  (if (and (> _returnvalue_8 0.0) (> _returnvalue_9 0.0))
    ;[1 1 1] Validate that path finding manager has been initialized
    (if (Utilities|IsValid (Variables|Default|GetPathFindingManager))
      ;[1 1 1] Make sure that the player position is within the bounds
      (if (and (< _returnvalue_8 (* _x_2 _griddisplacement)) (< _returnvalue_9 (* _y_2 _griddisplacement)))
        (bind _ismoving (CallFunction|CheckifPlayerIsMoving _returnvalue_7))
        (bind _output_get (Variables|Default|SetisPlayerMoving _ismoving))
        (if _output_get
          (CallFunction|ClearPaths))
        (Transformation|AddActorWorldOffset _returnvalue_7)))))

(event Input|MouseEvents|MouseWheelUp
  (params (Key :type Key%20Structure))
  ;[1 1 1] Controling zoom on the camera
  (:Pressed
    (Variables|Default|SetZoom (Math|Float|Clamp(Float) (+ (Variables|Default|GetZoom) -1e+02) 6e+02 3e+03))
    (Variables|/Script/Engine.SpringArmComponent|SetTargetArmLength (Variables|Default|GetSpringArm) (Variables|Default|GetZoom))))

(event Input|MouseEvents|MouseWheelDown
  (params (Key :type Key%20Structure))
  ;[1 1 1] Controling zoom on the camera
  (:Pressed
    (Variables|Default|SetZoom (Math|Float|Clamp(Float) (+ (Variables|Default|GetZoom) 1e+02) 6e+02 3e+03))
    (Variables|/Script/Engine.SpringArmComponent|SetTargetArmLength (Variables|Default|GetSpringArm) (Variables|Default|GetZoom))))

(fn ConstructionScript)

(fn SpawnWallsRandomly
  (CallFunction|DeleteWalls)
  ;[1 1 1] Go through walls to be spawned and set their position and then eventually spawn them
  (for _index (range 0 (Variables|/Game/SteeringActor/BP_PathFindingManager.BP_PathFindingManager_C|GetWallsPerSpawn (Variables|Default|GetPathFindingManager)))
    (bind (_returnvector _returnx _returny) (CallFunction|GenerateGridPosition))
    ;[1 1 1] Check that the new grid does not overlap any steering actors
    (for (_ _array_index) (Variables|Default|GetSteeringActors)
      (if (not (and (== _returnx (Math|Float|Round (.X (Math|Vector2D|BreakVector2D (Variables|/Game/SteeringActor/BP_SteeringActor.BP_SteeringActor_C|GetActorPos (Utilities|Array|Get(acopy) (Variables|Default|GetSteeringActors) _array_index)))))) (== (Math|Float|Round (.Y (Math|Vector2D|BreakVector2D (Variables|/Game/SteeringActor/BP_SteeringActor.BP_SteeringActor_C|GetActorPos (Utilities|Array|Get(acopy) (Variables|Default|GetSteeringActors) _array_index))))) _returny)))
        ;[1 1 1] Spawn wall and set its X and Y values on the grid
        (bind _returnvalue (Game|SpawnActorfromClass "/Game/Misc/BP_Wall.BP_Wall_C" (Math|Conversions|ToTransform(Vector) _returnvector) "Undefined" 0 0))
        ;[1 1 1] Set the Grid's position
        (bind (_outxval _outyval) (CallFunction|ValidateGridPosition _returnx _returny))
        (Variables|/Game/Misc/BP_Wall.BP_Wall_C|SetgridX _returnvalue _outxval)
        (Variables|/Game/Misc/BP_Wall.BP_Wall_C|SetgridY _returnvalue _outyval)
        (Utilities|Array|Add (Variables|Default|GetWalls) (Math|Vector2D|MakeVector2D (Math|Conversions|ToFloat(Integer) (Variables|/Game/Misc/BP_Wall.BP_Wall_C|GetgridX _returnvalue)) (Math|Conversions|ToFloat(Integer) (Variables|/Game/Misc/BP_Wall.BP_Wall_C|GetgridY _returnvalue))))))))

(fn AssignWallstoActors
  ;[1 1 1] Go and get all steering actors
  (bind _outactors (Actor|GetAllActorsOfClass "/Game/SteeringActor/BP_SteeringActor.BP_SteeringActor_C"))
  (bind _output_get (Variables|Default|SetSteeringActors _outactors))
  ;[1 1 1] Assign the walls to the given steering actors
  (for (_array_element _array_index) _output_get
    (Class|PathFindingActor|AddWalls _array_element (Variables|Default|GetWalls))
    (bind _returnvalue (Class|PathFindingActor|FindPath _array_element (Variables|/Game/SteeringActor/BP_SteeringActor.BP_SteeringActor_C|GetActorPos (Utilities|Array|Get(acopy) (Variables|Default|GetSteeringActors) _array_index)) (Variables|/Game/SteeringActor/BP_SteeringActor.BP_SteeringActor_C|GetPlayerPos (Utilities|Array|Get(acopy) (Variables|Default|GetSteeringActors) _array_index))))
    (Variables|/Game/SteeringActor/BP_SteeringActor.BP_SteeringActor_C|SetinputPath (Utilities|Array|Get(acopy) (Variables|Default|GetSteeringActors) _array_index) _returnvalue)
    (Default|SmoothPath (Utilities|Array|Get(acopy) (Variables|Default|GetSteeringActors) _array_index))
    (Variables|/Game/SteeringActor/BP_SteeringActor.BP_SteeringActor_C|SettempEndPos (Utilities|Array|Get(acopy) (Variables|Default|GetSteeringActors) _array_index) (Variables|/Game/SteeringActor/BP_SteeringActor.BP_SteeringActor_C|GetPlayerPos (Utilities|Array|Get(acopy) (Variables|Default|GetSteeringActors) _array_index)))
    (Variables|/Game/SteeringActor/BP_SteeringActor.BP_SteeringActor_C|SetreachedDestination (Utilities|Array|Get(acopy) (Variables|Default|GetSteeringActors) _array_index) true)))

(fn GenerateGridPosition
  (bind _pathfindingmanager (Variables|Default|GetPathFindingManager))
  (bind _griddisplacement (Variables|/Game/SteeringActor/BP_PathFindingManager.BP_PathFindingManager_C|GetGridDisplacement _pathfindingmanager))
  (bind _griddimensions (Variables|/Game/SteeringActor/BP_PathFindingManager.BP_PathFindingManager_C|GetGridDimensions _pathfindingmanager))
  (bind _returnvalue (Math|Float|Truncate _griddisplacement))
  (bind (_x _y) (Math|Vector2D|BreakVector2D _griddimensions))
  (bind _returnvalue_2 (Math|Float|Round _y))
  (bind _returnvalue_3 (Math|Float|Round _x))
  (bind _returnvalue_4 (- _returnvalue_2 1))
  (bind _returnvalue_5 (- _returnvalue_3 1))
  (bind _returnvalue_6 (Math|Random|RandomIntegerinRange 0 _returnvalue_5))
  (bind _returnvalue_7 (Math|Random|RandomIntegerinRange 0 _returnvalue_4))
  (return (Math|Vector|MakeVector (Math|Conversions|ToFloat(Integer) (* _returnvalue_6 _returnvalue)) (Math|Conversions|ToFloat(Integer) (* _returnvalue _returnvalue_7)) 5e+01) _returnvalue_6 _returnvalue_7))

(fn ClearPaths
  ;[1 1 1] Go through all steering actors and clear their paths
  (for _array_element (Variables|Default|GetSteeringActors)
    (Utilities|Array|Clear (Variables|/Script/PathFinding.PathFindingActor|GetPath _array_element))
    (bind _returnvalue (Class|PathFindingActor|FindPath _array_element (Variables|/Game/SteeringActor/BP_SteeringActor.BP_SteeringActor_C|GetActorPos _array_element) (Variables|/Game/SteeringActor/BP_SteeringActor.BP_SteeringActor_C|GetPlayerPos _array_element)))
    (if (Variables|/Game/SteeringActor/BP_SteeringActor.BP_SteeringActor_C|GetisSmoothing _array_element)
      (Variables|/Game/SteeringActor/BP_SteeringActor.BP_SteeringActor_C|SetinputPath _array_element _returnvalue)
      (Default|SmoothPath _array_element)
      (else
        (Class|PathFindingActor|SetPathtoFollow _array_element _returnvalue)))
    (Variables|/Game/SteeringActor/BP_SteeringActor.BP_SteeringActor_C|SettempEndPos _array_element (Variables|/Game/SteeringActor/BP_SteeringActor.BP_SteeringActor_C|GetPlayerPos _array_element))
    (Variables|/Game/SteeringActor/BP_SteeringActor.BP_SteeringActor_C|SetreachedDestination _array_element true)))

(fn ValidateGridPosition
  (params (xVal :type Integer) (yVal :type Integer))
  (bind _pathfindingmanager (Variables|Default|GetPathFindingManager))
  (bind _griddimensions (Variables|/Game/SteeringActor/BP_PathFindingManager.BP_PathFindingManager_C|GetGridDimensions _pathfindingmanager))
  (bind (_x _y) (Math|Vector2D|BreakVector2D _griddimensions))
  ;[1 1 1] Check and make sure that the wall is not outside of the grid
  (bind _output_get (Variables|Default|SettmpXVal xVal))
  (if (|({E3F1A237-4E44-CCB2-E941-81A7ADBA980E}>=dimension) (Math|Float|Round _x))
    (if (== _output_get 0)
      _
      (else
        (Variables|Default|SettmpXVal (- (Variables|Default|GettmpXVal) 1)))))
  (bind _output_get_2 (Variables|Default|SettmpYVal yVal))
  (if (|({2DDC072E-4A8D-4732-9B9A-988657B38540}>=dimension) (Math|Float|Round _y))
    (if (== _output_get_2 0)
      _
      (else
        (Variables|Default|SettmpYVal (- (Variables|Default|GettmpYVal) 1)))))
  (return (Variables|Default|GettmpXVal) (Variables|Default|GettmpYVal)))

(fn ValidateNewPositionOfSteeringActor
  (bind _pathfindingmanager (Variables|Default|GetPathFindingManager))
  (bind _pathfindingmanager_2 (Variables|Default|GetPathFindingManager))
  (bind _griddisplacement (Variables|/Game/SteeringActor/BP_PathFindingManager.BP_PathFindingManager_C|GetGridDisplacement _pathfindingmanager))
  (bind _griddimensions (Variables|/Game/SteeringActor/BP_PathFindingManager.BP_PathFindingManager_C|GetGridDimensions _pathfindingmanager_2))
  (bind (_x _y) (Math|Vector2D|BreakVector2D _griddimensions))
  (bind _returnvalue (Math|Float|Truncate _griddisplacement))
  (bind _returnvalue_2 (Math|Float|Truncate _x))
  (bind _returnvalue_3 (Math|Float|Truncate _y))
  (bind _returnvalue_4 (- _returnvalue_2 1))
  (bind _returnvalue_5 (- _returnvalue_3 1))
  (bind _returnvalue_6 (Math|Random|RandomIntegerinRange 0 _returnvalue_4))
  (bind _returnvalue_7 (Math|Random|RandomIntegerinRange 0 _returnvalue_5))
  ;[1 1 1] Make sure that the proposed steering actor does no overlap a wall
  (for _array_element (Variables|Default|GetWalls)
    (if (Math|Vector|Equal(Vector) _array_element (Math|Vector2D|MakeVector2D (Math|Conversions|ToFloat(Integer) _returnvalue_6) (Math|Conversions|ToFloat(Integer) _returnvalue_7)) 0.0001)
      (return true "0, 0, 0")))
  (return false (Math|Vector|MakeVector (Math|Conversions|ToFloat(Integer) (* _returnvalue_6 _returnvalue)) (Math|Conversions|ToFloat(Integer) (* _returnvalue_7 _returnvalue)) 7e+01)))

(fn CheckifPlayerIsMoving
  (params (MovementVector :type Vector))
  (bind (_x _y _z) (Math|Vector|BreakVector MovementVector))
  (return (Math|Boolean|ORBoolean (> _x 0.0) (> _y 0.0) (> _z 0.0))))

(fn SpawnSteeringActors
  ;[1 1 1] Spawns steering actors in random locations on the map
  (bind (_isoverlapping _newposition) (CallFunction|ValidateNewPositionOfSteeringActor :!label _label))
  (if _isoverlapping
    (goto _label)
    (else
      (Game|SpawnActorfromClass "/Game/SteeringActor/BP_SteeringActor.BP_SteeringActor_C" (Math|Conversions|ToTransform(Vector) _newposition) "Undefined" 0 0)
      (CallFunction|AssignWallstoActors))))

(fn DeleteWalls
  (Utilities|Array|Clear (Variables|Default|GetWalls))
  ;[1 1 1] Destroy previous walls
  (bind _outactors (Actor|GetAllActorsOfClass "/Game/Misc/BP_Wall.BP_Wall_C"))
  (for _array_element _outactors
    (Actor|DestroyActor _array_element))
  (bind _outactors_2 (Actor|GetAllActorsOfClass "/Game/SteeringActor/BP_SteeringActor.BP_SteeringActor_C"))
  (bind _output_get (Variables|Default|SetSteeringActors _outactors_2))
  (for _array_element_2 _output_get
    (Class|PathFindingActor|ResetWalls _array_element_2))
  (return))

(fn SwitchPathfindingAlgorithms
  (params (isUsingDjikstra :type Boolean))
  (for _array_element (Variables|Default|GetSteeringActors)
    (Variables|/Script/PathFinding.PathFindingActor|SetuseDjikstra _array_element isUsingDjikstra)))

(fn SwitchPathType
  (params (pathSmoothed :type Boolean))
  (for _array_element (Variables|Default|GetSteeringActors)
    (Variables|/Game/SteeringActor/BP_SteeringActor.BP_SteeringActor_C|SetisSmoothing _array_element pathSmoothed)))