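; BP_Wall is a wall actor with no running logic: its construction script is empty and its only event graph nodes are never executed.
; Those disconnected nodes would derive GridX and GridY by truncating the actor's X and Y location and dividing by SpacingBetweenGrids, mapping the wall onto a grid cell.
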(fn ConstructionScript)